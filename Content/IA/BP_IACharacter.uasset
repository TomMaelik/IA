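; BP_IACharacter is an AI-controlled character that runs the BT_Test behavior tree on BeginPlay through its AIController.
; Its AIPerception component reacts only to BP_ThirdPersonCharacter, printing debug strings depending on whether the stimulus was successfully sensed.
; An unconnected AIMoveTo loop for wandering between random reachable points remains in the event graph but never runs.
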(event `self.ReceiveBeginPlay`
  ;[0.1083 0.4844 0.01546 0.5] Setup a faire
  (bind _asaicontroller (cast `AIController` (`self.GetController`)))
  (`AIController.RunBehaviorTree` _asaicontroller "/Game/IA/BT_Test.BT_Test"))

(event `self.AIPerception.OnTargetPerceptionUpdated`
  (params (Actor :type "Actor Object Reference") (Stimulus :type "AIStimulus Structure"))
  (cast `/Game/ThirdPerson/Blueprints/BP_ThirdPersonCharacter` Actor)
  (if Stimulus_bSuccessfullySensed
    (`KismetSystemLibrary.PrintString` "Hello")
    (else
      (`KismetSystemLibrary.PrintString` "4"))))

(fn `UserConstructionScript`)